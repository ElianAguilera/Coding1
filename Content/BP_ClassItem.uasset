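; Item Blueprint with a name, elemental type and damage value that prints a test of elemental damage on BeginPlay.
; Constructor, a function called from BeginPlay, picks a random name from a hardcoded list if Name is still the default.
; GetDamage finds opposite elements with modulo-4 enum arithmetic, returning zero for an opposite victim and base Damage otherwise.
; An unconnected Earth switch with double damage remains unused.
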(event `self.ReceiveBeginPlay`
  (`self.Constructor`)
  (`KismetSystemLibrary.PrintString` (`KismetStringLibrary.Concat_StrStr` "Hello! My name is " (`self.Name`)) true true (struct :`R` 1.0 :`G` 0.751827 :`A` 1.0) 20.0)
  (bind _damage (`self.GetDamage` "NewEnumerator3"))
  (`KismetSystemLibrary.PrintString` (`KismetStringLibrary.Concat_StrStr` "Our elem type is  " (`|GetEnumeratorNameAsString` (`self.ElementalType`)) ", victim is air, damage = " (`KismetStringLibrary.Conv_IntToString` _damage)) true true (struct :`R` 1.0 :`B` 0.013789 :`A` 1.0) 10.0))

(fn `Constructor`
  (bind _array (`|MakeArray` "Elian" "Aaron" "Dameron"))
  (if (`KismetStringLibrary.EqualEqual_StrStr` (`self.Name`) "Item")
    (`KismetArrayLibrary.Array_Shuffle` _array)
    (set `self.Name` (`|GetArrayItem` _array (`KismetMathLibrary.RandomIntegerInRange` 0 (- (`KismetArrayLibrary.Array_Length` _array) 0))))))

(fn `GetDamage`
  (params (`Victim Elem Type` :type "/Game/ElementalType Enum" :default "NewEnumerator1"))
  (returns (Damage :type Integer))
  (locals (ReturnedDamage :type Integer :default 0))
  (set `local.ReturnedDamage` (`self.Damage`))
  (if (== (mod (+ `Victim Elem Type` 2) 4) (`KismetMathLibrary.Conv_ByteToInt` (`self.ElementalType`)))
    (set `local.ReturnedDamage` (* (`self.Damage`) 0)))
  (return (`local.ReturnedDamage`)))

(fn `UserConstructionScript`)