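; Function-practice Blueprint that prints colored on-screen debug messages on BeginPlay.
; A Say event prints in random colors, and CountToNumber calls it in a loop with durations that grow per index.
; It then prints each array string colored by GetColorByNameLength: white at five or more characters, otherwise grayscale via a custom NormalizeFromRange.
; The black branch for long strings is unreachable, and the helper's math is not a true normalization.
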(event `self.ReceiveBeginPlay`
  (`KismetSystemLibrary.PrintString` "We are exploring functions today!" true true (struct :`G` 0.66 :`B` 1.0 :`A` 1.0) 5.0)
  (`self.Say` "Hello My Goat")
  (`self.CountToNumber` 10)
  (for _array_element (`self.NewVar`)
    (bind _output (`self.GetColorByNameLength` _array_element))
    (`KismetSystemLibrary.PrintString` _array_element true true _output 10.0)))

(event `Say`
  (params (InString :type String :default "Hello My Goat") (Duration :type "Float (single-precision)" :default 5.0))
  (`KismetSystemLibrary.PrintString` InString true true (make `LinearColor` (`KismetMathLibrary.RandomFloat`) (`KismetMathLibrary.RandomFloat`) (`KismetMathLibrary.RandomFloat`) 1.0) Duration))

(fn `CountToNumber`
  (params (Number :type Integer :default 10))
  (for _index (range (+ Number 1))
    (`self.Say` (`KismetStringLibrary.Conv_IntToString` _index) (+ 5.0 (* _index 0.1))))
  (return) ; Continues that chain
)

(fn `GetColorByNameLength`
  (params (Input :type String))
  (returns (Output :type "LinearColor Structure"))
  (locals (`Output Color` :type "LinearColor Structure"))
  (bind _returnvalue (`KismetStringLibrary.Len` Input))
  (bind _returnvalue_2 (* (`self.NormalizeFromRange` 5.0 10.0 (`KismetMathLibrary.Conv_IntToDouble` _returnvalue)) 0.2))
  (if (<= 5 _returnvalue)
    (set `local.Output Color` (make `LinearColor` 1.0 1.0 1.0 1.0))
    (elif (>= _returnvalue 10)
      (set `local.Output Color` (make `LinearColor` 0.0 0.0 0.0 1.0))
      (else
        (set `local.Output Color` (make `LinearColor` _returnvalue_2 _returnvalue_2 _returnvalue_2 1.0)))))
  (return (`local.Output Color`)))

(fn `NormalizeFromRange`
  (params (Min :type "Float (double-precision)") (Max :type "Float (double-precision)") (Input :type "Float (double-precision)"))
  (returns (ReturnValue :type "Float (double-precision)"))
  (bind _returnvalue (- Min Input))
  (return (* _returnvalue (/ _returnvalue (- Max 0.0)))))

(fn `UserConstructionScript`)