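; Enemy actor that takes a random name and team material on BeginPlay unless already set, applying the material to its cylinder and sphere meshes.
; A looping delay polls Health and destroys the actor once it reaches zero or below.
; Capsule overlap with BP_ThirdPersonCharacter sets Health negative, so contact is lethal.
; The held item's element-based damage is queried but multiplied by zero, so it has no effect.
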(event `self.ReceiveBeginPlay`
  (bind _names (`self.Names`))
  (bind _color (`self.Color`))
  (`|ExecutionSequence`
    (:`then_0`
      ;[0.2574 0.4958 0.2513] after .2 seconds, check to see if actor health is <= 0 if it is destroy actor
      (`KismetSystemLibrary.Delay` 0.2 :!label _label)
      (if (<= (`self.Health`) 0.0)
        (`self.K2_DestroyActor`)
        (else
          (goto _label))))
    (:`then_1`
      (if (== (`self.Enemy Name`) "None")
        (`KismetArrayLibrary.Array_Shuffle` _names)
        (set `self.Enemy Name` (`|GetArrayItem` _names)) ; set the randomized name
      )
      (`KismetSystemLibrary.PrintString` (`KismetStringLibrary.Concat_StrStr` (`KismetStringLibrary.Conv_NameToString` (`self.Enemy Name`)) " exists!") true true (struct :`G` 0.66 :`B` 1.0 :`A` 1.0) 20.0))
    (:`then_2`
      (`/Engine/EditorBlueprintResources/StandardMacros.IsValid` (`self.Enemy Team Material`)
        (:`Is Valid`
          (`KismetSystemLibrary.PrintString` "A meterial Has been set!" true true (struct :`R` 1.0 :`G` 1.0 :`B` 1.0 :`A` 1.0) 5.0))
        (:`Is Not Valid`
          (`KismetSystemLibrary.PrintString` "lets pick a random material!" true true (struct :`R` 1.0 :`G` 1.0 :`B` 1.0 :`A` 1.0) 5.0)
          (`KismetArrayLibrary.Array_Shuffle` _color) ; Shuffle the materials
          (set `self.Enemy Team Material` (`|GetArrayItem` _color))))
      (`PrimitiveComponent.SetMaterial` (`self.Cylinder`) 0 (`self.Enemy Team Material`)) ; select the material that was selected
      (`PrimitiveComponent.SetMaterial` (`self.Sphere`) 0 (`self.Enemy Team Material`)))))

(event `self.CapsuleCollision.OnComponentBeginOverlap`
  (params (OverlappedComponent :type "PrimitiveComponent Object Reference") (OtherActor :type "Actor Object Reference") (OtherComp :type "PrimitiveComponent Object Reference") (OtherBodyIndex :type Integer) (bFromSweep :type Boolean) (SweepResult :type "HitResult Structure (by ref)"))
  (bind _asbp_third_person_character (cast `/Game/ThirdPerson/Blueprints/BP_ThirdPersonCharacter` OtherActor))
  (set `self.Health` -1.0)
  (bind _damage (`/Game/BP_ClassItem.GetDamage` (`/Game/ThirdPerson/Blueprints/BP_ThirdPersonCharacter.heldItem2` _asbp_third_person_character) (`self.ElemType`)))
  (bind _output_get (set `self.Health` (- (`self.Health`) (* (`KismetMathLibrary.Conv_IntToDouble` _damage) 0.0))))
  (`KismetSystemLibrary.PrintString` (`KismetStringLibrary.Concat_StrStr` "health is now " (`KismetStringLibrary.Conv_DoubleToString` _output_get))))

(fn `UserConstructionScript`)