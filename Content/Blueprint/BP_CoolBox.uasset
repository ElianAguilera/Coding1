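; BP_CoolBox is a test actor with a Cube component that prints debug information when play begins.
; BeginPlay prints the actor's display name with an existence message, then the cube's world location, then that location offset upward along Z, without moving the cube.
; Overlap, Tick and the construction script are empty.
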(event `self.ReceiveBeginPlay`
  (bind _returnvalue (`SceneComponent.K2_GetComponentLocation` (`self.Cube`)))
  (`KismetSystemLibrary.PrintString` (`KismetStringLibrary.Concat_StrStr` (`KismetSystemLibrary.GetDisplayName` self) " exists!") true true (struct :`R` 1.0 :`G` 0.008255 :`B` 0.095915 :`A` 1.0) 10.0)
  (`KismetSystemLibrary.PrintString` (`KismetStringLibrary.Conv_VectorToString` _returnvalue) true true (struct :`R` 0.20256 :`G` 1.0 :`B` 0.082339 :`A` 1.0) 10.0)
  (`KismetSystemLibrary.PrintString` (`KismetStringLibrary.Conv_VectorToString` (+ _returnvalue (0.0 0.0 200.0)))))

(fn `UserConstructionScript`)